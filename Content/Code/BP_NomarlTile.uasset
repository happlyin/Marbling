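; BP_NomarlTile is a purchasable board tile that tracks its owner, payment amount and purchase price.
; The Construction Script creates a dynamic material instance on the NomarlTile component.
; ChangeOwner swaps that material's TileColor texture and records the owner number.
; SetBase initializes the base, current and purchase amounts, then calls ChangeOwner to reset the tile to unowned; the event graph is empty.
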(event EventBeginPlay)

(event Collision|EventActorBeginOverlap
  (params (OtherActor :type Actor%20Object%20Reference)))

(event EventTick
  (params (DeltaSeconds :type Float%20%28single-precision%29)))

(fn ConstructionScript
  (bind _returnvalue (Rendering|Material|CreateDynamicMaterialInstance (Variables|Default|GetNomarlTile) 0 0 "None" :!class /Script/Engine.PrimitiveComponent))
  (Variables|Default|SetMaterial_Instance _returnvalue))

(fn ChangeOwner
  (params (Texture :type Texture%202D%20Object%20Reference) (OwnerNumber :type Integer))
  (Rendering|Material|SetTextureParameterValue (Variables|Default|GetMaterial_Instance) "TileColor" Texture)
  (Variables|Default|SetNowOwner OwnerNumber))

(fn SetBase
  (params (BassPay :type Integer) (BuyPay :type Integer))
  (bind _output_get (Variables|Default|SetBasePay BassPay))
  (Variables|Default|SetNowPay _output_get)
  (Variables|Default|SetBuyPay BuyPay)
  (CallFunction|ChangeOwner "/Game/3D_Files/Tile/Texture_NomralTileNo.Texture_NomralTileNo" -1))