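; BP_GoCard is a card actor that holds a random number and can change its face texture and flip.
; The construction script creates a dynamic material instance on the RandomCard component, whose Texture parameter SetTexture overwrites.
; ReSetNumber rolls MyNumber from 0 to 5 and runs at BeginPlay, while Rotation180 turns RandomCard half a turn.
; Nothing in this Blueprint links the number to the texture or calls the texture and rotation functions.
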(event EventBeginPlay
  (CallFunction|ReSetNumber))

(event Collision|EventActorBeginOverlap
  (params (OtherActor :type Actor%20Object%20Reference)))

(event EventTick
  (params (DeltaSeconds :type Float%20%28single-precision%29)))

(fn ConstructionScript
  (bind _returnvalue (Rendering|Material|CreateDynamicMaterialInstance (Variables|Default|GetRandomCard) 0 0 "None" :!class /Script/Engine.PrimitiveComponent))
  (Variables|Default|SetMaterial_Instance _returnvalue))

(fn SetTexture
  (params (Texture :type Texture%202D%20Object%20Reference))
  (Rendering|Material|SetTextureParameterValue (Variables|Default|GetMaterial_Instance) "Texture" Texture))

(fn Rotation180
  (Transformation|AddRelativeRotation (Variables|Default|GetRandomCard) "180.000000, 0, 0" false false))

(fn ReSetNumber
  (Variables|Default|SetmyNumber (Math|Random|RandomInteger 6)))