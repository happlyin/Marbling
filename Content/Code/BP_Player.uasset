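; BP_Player is a player pawn or piece that holds its money, player number and position vector.
; On BeginPlay it sets its current money to a fixed starting amount.
; The construction script creates a dynamic material on the Character component, which SetPlayerColor uses to swap the PlayerColor texture.
; Simple setters store the player number and start vector, with no movement or spending logic here.
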(event EventBeginPlay
  (Variables|Default|SetMoneyStandard 10000)
  (Variables|Default|SetNowMoney (Variables|Default|GetMoneyStandard)))

(event Collision|EventActorBeginOverlap
  (params (OtherActor :type Actor%20Object%20Reference)))

(event EventTick
  (params (DeltaSeconds :type Float%20%28single-precision%29)))

(fn ConstructionScript
  (bind _returnvalue (Rendering|Material|CreateDynamicMaterialInstance (Variables|Default|GetCharacter) 0 0 "None" :!class /Script/Engine.PrimitiveComponent))
  (Variables|Default|SetMaterial_Instance _returnvalue))

(fn SetPlayerColor
  (params (Texture :type Texture%202D%20Object%20Reference))
  (Rendering|Material|SetTextureParameterValue (Variables|Default|GetMaterial_Instance) "PlayerColor" Texture))

(fn SetPlayerNumber
  (params (PlayerNumber :type Integer))
  (Variables|Default|SetPlayerNumber PlayerNumber))

(fn SetStarVector3
  (params (StartVector3 :type Vector))
  (Variables|Default|SetNowMyVector StartVector3))