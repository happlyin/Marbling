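; BP_Players is a player piece for what appears to be a tile-based board game, tracking player number, tile position and money.
; Construction creates a dynamic material on the Character component, whose PlayerColor texture parameter sets each player's look.
; Setters move the piece and advance its tile count, while Rotation turns it 90 degrees.
; ReSetPlayerInfo reapplies color, number, position and starting money, but its additive tile call leaves the tile number unchanged.
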(event EventBeginPlay
  (Variables|Default|SetMoneyStandard 10000)
  (Variables|Default|SetNowMoney (Variables|Default|GetMoneyStandard)))

(event Collision|EventActorBeginOverlap
  (params (OtherActor :type Actor%20Object%20Reference)))

(event EventTick
  (params (DeltaSeconds :type Float%20%28single-precision%29)))

(fn ConstructionScript
  (bind _returnvalue (Rendering|Material|CreateDynamicMaterialInstance (Variables|Default|GetCharacter) 0 0 "None" :!class /Script/Engine.PrimitiveComponent))
  (Variables|Default|SetMaterial_Instance _returnvalue))

(fn SetPlayerColor
  (params (Texture :type Texture%202D%20Object%20Reference))
  (Rendering|Material|SetTextureParameterValue (Variables|Default|GetMaterial_Instance) "PlayerColor" Texture))

(fn SetPlayerNumber
  (params (PlayerNumber :type Integer))
  (Variables|Default|SetPlayerNumber PlayerNumber))

(fn SetPlayerPos
  (params (StartVector3 :type Vector))
  (bind _output_get (Variables|Default|SetNowMyVector StartVector3))
  (Transformation|SetWorldLocationAndRotation (Variables|Default|GetCharacter) _output_get "0, 0, 0" false false))

(fn SetNowTileNumber
  (params (ForwardCount :type Integer))
  (Variables|Default|SetNowTileNumber (+ ForwardCount (Variables|Default|GetNowTileNumber))))

(fn ReSetPlayerInfo
  (params (Texture :type Texture%202D%20Object%20Reference) (PlayerNumber :type Integer) (StartVector :type Vector))
  (CallFunction|SetPlayerColor Texture)
  (CallFunction|SetPlayerNumber PlayerNumber)
  (CallFunction|SetPlayerPos StartVector)
  (CallFunction|SetNowTileNumber)
  (Variables|Default|SetNowMoney (Variables|Default|GetMoneyStandard)))

(fn Rotation
  (Transformation|AddWorldRotation (Variables|Default|GetCharacter) "0,90.000000, 0" false false))